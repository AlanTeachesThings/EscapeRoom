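; R_BaseObject_BP is an interactable object Blueprint that relays highlight and interaction events to its R_Interaction components.
; On BeginPlay it caches every R_Interaction component it owns.
; AddHighlights, RemoveHighlights and OnBeginInteraction each loop over that array to toggle highlights or call OnBeginMasterInteraction.
; The instigating character is not passed on to the components, and the construction script is empty.
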(event Custom|AddHighlights
  (for _array_element (Variables|Default|GetInteractionComponents)
    (Default|AddHighlight _array_element)))

(event Custom|RemoveHighlights
  (for _array_element (Variables|Default|GetInteractionComponents)
    (Default|RemoveHighlight _array_element)))

(event Custom|OnBeginInteraction
  (params (InstigatingCharacter :type BP%20First%20Person%20Character%20Object%20Reference))
  (for _array_element (Variables|Default|GetInteractionComponents)
    (Default|OnBeginMasterInteraction _array_element)))

(event EventBeginPlay
  (Variables|Default|SetInteractionComponents (Actor|GetComponentsByClass "/Game/RefactorTesting/R_Interaction.R_Interaction_C")))

(fn ConstructionScript)