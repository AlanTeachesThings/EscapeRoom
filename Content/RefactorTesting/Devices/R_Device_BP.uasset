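; Interactable device actor that, when unlocked, hands the player's focus to its R_Interaction components, starting with the lowest-priority-value one that captures attention.
; Directional input hops between components via named Up/Down/Left/Right links under a cooldown, otherwise passing through to the active component.
; Activating a component updates highlight and player UI, then blends to its child camera, the device's camera or the player's.
; UnlockedBy lock events are bound, but their handler is empty.
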(event Custom|AddHighlights
  ;[0.15 0.15 0.15 0.5] Add Highlights to all components
  (for _array_element (Variables|Default|GetInteractionComponents)
    (Default|AddHighlight _array_element)))

(event Custom|RemoveHighlights
  ;[0.15 0.15 0.15 0.5] Add Highlights to all components
  (for _array_element (Variables|Default|GetInteractionComponents)
    (Default|RemoveHighlight _array_element)))

(event Custom|SetInteractionComponentAsActive
  (params (New%20Interaction%20Component :type R%20Interaction%20Object%20Reference))
  (bind _interactioncameracomponent (CallFunction|CurrentInteractionCamera))
  (bind _returnvalue (Actor|GetComponentbyClass "/Script/Engine.CameraComponent"))
  (bind _currentinstigatingcharacter (Variables|Default|GetCurrentInstigatingCharacter))
  (bind _currentinstigatingcharacter_2 (Variables|Default|GetCurrentInstigatingCharacter))
  ;[0.15 0.15 0.15 0.5] Set new Interaction Component: Remove old Highlight if necesary, add new Highlight, display "Back Out" UI and Cursor if appropriate, then check for cameras on interaction or Device and adjust as appropriate
  (Utilities|FlowControl|Sequence
    (:then_0
      ;;[1 1 1] Remove highlight from last interaction (if applicable) and then highlight new one
      (Utilities|IsValid (Variables|Default|GetCurrentInteractionComponent)
        (:Is%20Valid
          (Default|RemoveHighlight (Variables|Default|GetCurrentInteractionComponent)))
        (:Is%20Not%20Valid
          _))
      (bind _output_get (Variables|Default|SetCurrentInteractionComponent New%20Interaction%20Component))
      (Default|AddHighlight _output_get))
    (:then_1
      ;;[1 1 1] Hide the reticle, show the "back out" UI and (if using Keyboard Controls) show Mouse Cursor
      (Default|ShowBackOut _currentinstigatingcharacter_2)
      (Default|HideReticle _currentinstigatingcharacter_2)
      (Variables|/Game/RefactorTesting/Core/EscapeRoom_Character.EscapeRoom_Character_C|GetisUsingGamepadControls _currentinstigatingcharacter_2
        (:then)
        (:else
          (Default|ShowCursor _currentinstigatingcharacter_2))))
    (:then_2
      ;;[1 1 1] If Interaction contains a camera, use that. If not, check if device uses camera and use that. If not, revert to player cam
      (Utilities|IsValid _interactioncameracomponent
        (:Is%20Valid
          (CallFunction|MakeActiveCameraComponent _interactioncameracomponent 0.25 "VTBlend_Linear" 0.0 false))
        (:Is%20Not%20Valid
          (Utilities|IsValid _returnvalue
            (:Is%20Valid
              (CallFunction|MakeActiveCameraComponent _returnvalue 0.25 "VTBlend_Linear" 0.0 false))
            (:Is%20Not%20Valid
              (Default|SetNewCamera _currentinstigatingcharacter _currentinstigatingcharacter 0.25 "VTBlend_Linear" 0.0 false))))))
    (:then_3
      ;;[1 1 1] Now begin the Interaction!
      (Default|StartInteraction (Variables|Default|GetCurrentInstigatingCharacter) self (Variables|Default|GetCurrentInteractionComponent)))))

(event Custom|EndExamine
  (params (InstigatingCharacter :type BP%20First%20Person%20Character%20Object%20Reference)))

(event Custom|EndInteraction
  ;[0.15 0.15 0.15 0.5] Intearction Ends
  (Default|EndInteraction (Variables|Default|GetCurrentInstigatingCharacter))
  (Default|HideBackOut (Variables|Default|GetCurrentInstigatingCharacter))
  (Default|HideCursor (Variables|Default|GetCurrentInstigatingCharacter))
  (Default|HideReticle (Variables|Default|GetCurrentInstigatingCharacter))
  (Variables|Default|SetCurrentInstigatingCharacter 0))

(event Custom|LockUpdate
  (params (isLocked :type Boolean))
  (Default|CallLockUpdateEvent isLocked))

(event Custom|OnLockUpdate
  (params (isLocked :type Boolean))
  ;[0.15 0.15 0.15 0.5] Begin Play
)

(event Custom|InteractStart
  (params (InstigatingCharacter :type Escape%20Room%20Character%20Object%20Reference))
  (if (not (Variables|Default|GetisLocked))
    (CallFunction|OnBeginInteraction InstigatingCharacter)))

(event Custom|InteractDirectionalControl
  (params (ControlValues :type Vector%202D%20Structure) (InstigatingCharacter :type Escape%20Room%20Character%20Object%20Reference))
  (bind _x (Math|Vector2D|BreakVector2D ControlValues))
  (bind _y (Math|Vector2D|BreakVector2D ControlValues))
  (bind _currentinteractioncomponent (Variables|Default|GetCurrentInteractionComponent))
  (bind _interactionnavigation (Variables|/Game/RefactorTesting/Interactions/R_Interaction.R_Interaction_C|GetInteractionNavigation _currentinteractioncomponent))
  (bind (_interactioncomponent _componentfound) (CallFunction|GetComponentbyName (.right _interactionnavigation)))
  (bind (_interactioncomponent_2 _componentfound_2) (CallFunction|GetComponentbyName (.left _interactionnavigation)))
  (bind (_interactioncomponent_3 _componentfound_3) (CallFunction|GetComponentbyName (.up _interactionnavigation)))
  (bind (_interactioncomponent_4 _componentfound_4) (CallFunction|GetComponentbyName (.down _interactionnavigation)))
  (Utilities|IsValid (Variables|Default|GetCurrentInteractionComponent)
    (:Is%20Valid
      (Utilities|FlowControl|Sequence
        (:then_0
          (if (Math|Boolean|ANDBoolean (> _y 0.0) _componentfound_3 (> (Variables|Default|GetMoveCooldown) 1.0))
            (CallFunction|SetInteractionComponentasActive _interactioncomponent_3)
            (Variables|Default|SetMoveCooldown 0.0)
            (elif (Math|Boolean|ANDBoolean (< _y 0.0) _componentfound_4 (> (Variables|Default|GetMoveCooldown) 1.0))
              (CallFunction|SetInteractionComponentasActive _interactioncomponent_4)
              (Variables|Default|SetMoveCooldown 0.0)
              (else
                (Default|InteractDirectionalControl (Variables|Default|GetCurrentInteractionComponent) (Math|Vector2D|MakeVector2D 0.0 _y) InstigatingCharacter)))))
        (:then_1
          (if (Math|Boolean|ANDBoolean (< _x 0.0) _componentfound_2 (> (Variables|Default|GetMoveCooldown) 1.0))
            (CallFunction|SetInteractionComponentasActive _interactioncomponent_2)
            (Variables|Default|SetMoveCooldown 0.0)
            (elif (Math|Boolean|ANDBoolean (> _x 0.0) _componentfound (> (Variables|Default|GetMoveCooldown) 1.0))
              (CallFunction|SetInteractionComponentasActive _interactioncomponent)
              (Variables|Default|SetMoveCooldown 0.0)
              (else
                (Default|InteractDirectionalControl (Variables|Default|GetCurrentInteractionComponent) (Math|Vector2D|MakeVector2D _x 0.0))))))))))

(event Custom|InteractBack
  (params (InstigatingCharacter :type Escape%20Room%20Character%20Object%20Reference))
  (CallFunction|EndInteraction))

(event Custom|InteractPressTick
  (params (InstigatingCharacter :type Escape%20Room%20Character%20Object%20Reference)))

(event Custom|InteractPressStart
  (params (InstigatingCharacter :type Escape%20Room%20Character%20Object%20Reference)))

(event Custom|OnBeginInteraction
  (params (InstigatingCharacter :type Escape%20Room%20Character%20Object%20Reference))
  (bind _lowestpriorityinteraction (CallFunction|GetLowestPriorityInteraction))
  ;[0.15 0.15 0.15 0.5] Interaction Begins
  (Variables|Default|SetCurrentInstigatingCharacter InstigatingCharacter)
  (Utilities|FlowControl|Sequence
    (:then_0
      ;;[1 1 1] Remove highlights from all components
      (for _array_element (Variables|Default|GetInteractionComponents)
        (Default|RemoveHighlight _array_element)))
    (:then_1
      ;;[1 1 1] Call Begin Parent Interaction on all Interaction Components
      (for _array_element_2 (Variables|Default|GetInteractionComponents)
        (Default|OnBeginParentInteraction _array_element_2)))
    (:then_2
      ;;[1 1 1] Find Component with lowest interaction priority which also captures player, set that as current interaction
      (Utilities|IsValid _lowestpriorityinteraction
        (:Is%20Valid
          (CallFunction|SetInteractionComponentasActive _lowestpriorityinteraction))
        (:Is%20Not%20Valid
          (CallFunction|EndInteraction))))))

(event Custom|InteractPressEnd
  (params (InstigatingCharacter :type Escape%20Room%20Character%20Object%20Reference)))

(event Custom|Examine
  (params (InstigatingCharacter :type BP%20First%20Person%20Character%20Object%20Reference)))

(event EventTick
  (params (DeltaSeconds :type Float%20%28single-precision%29))
  ;[0.15 0.15 0.15 0.5] Tick
  (Variables|Default|SetMoveCooldown (+ DeltaSeconds (Variables|Default|GetMoveCooldown)))
  (|CallParentFunction DeltaSeconds))

(event EventBeginPlay
  ;[0.15 0.15 0.15 0.5] Begin Play
  (Utilities|FlowControl|Sequence
    (:then_0
      (Variables|Default|SetInteractionComponents (Actor|GetComponentsByClass "/Game/RefactorTesting/Interactions/R_Interaction.R_Interaction_C")))
    (:then_1
      (for _array_element (Variables|Default|GetUnlockedBy)
        (EventDispatchers|BindEventtoLockUpdateEvent _array_element (delegate Custom|OnLockUpdate))))))

(fn ConstructionScript)

(fn GetLowestPriorityInteraction
  (LocalVariables|SetLowestPriorityInteractionLocal 0)
  (LocalVariables|SetLowestPriorityDiscovered 2147483647)
  (for _array_element (Variables|Default|GetInteractionComponents)
    (if (and (< (Variables|/Game/RefactorTesting/Interactions/R_Interaction.R_Interaction_C|GetInteractionPriority _array_element) (LocalVariables|GetLowestPriorityDiscovered)) (Variables|/Game/RefactorTesting/Interactions/R_Interaction.R_Interaction_C|GetCapturesAttention _array_element))
      (LocalVariables|SetLowestPriorityDiscovered (Variables|/Game/RefactorTesting/Interactions/R_Interaction.R_Interaction_C|GetInteractionPriority _array_element))
      (LocalVariables|SetLowestPriorityInteractionLocal _array_element)))
  (return (LocalVariables|GetLowestPriorityInteractionLocal)))

(fn CheckforPlayerCapture
  (LocalVariables|SetShouldCapturePlayerLocal false)
  (for _array_element (Variables|Default|GetInteractionComponents)
    (if (Variables|/Game/RefactorTesting/Interactions/R_Interaction.R_Interaction_C|GetCapturesAttention _array_element)
      (LocalVariables|SetShouldCapturePlayerLocal true)))
  (return (LocalVariables|GetShouldCapturePlayerLocal)))

(fn CurrentInteractionCamera
  (LocalVariables|SetCameraComponentLocal 0)
  (for _array_element (Components|GetChildrenComponents (Variables|Default|GetCurrentInteractionComponent) true)
    (bind _ascamera_component (Utilities|Casting|CastToCameraComponent _array_element))
    (LocalVariables|SetCameraComponentLocal _ascamera_component))
  (return (LocalVariables|GetCameraComponentLocal)))

(fn MakeActiveCameraComponent
  (params (CameraComponentToMakeActive :type Camera%20Component%20Object%20Reference) (BlendTime :type Float%20%28single-precision%29) (BlendFunc :type EViewTargetBlendFunction%20Enum :default "VTBlend_Linear") (BlendExp :type Float%20%28single-precision%29) (bLockOutgoing :type Boolean))
  (for _array_element (Actor|GetComponentsByClass "/Script/Engine.CameraComponent")
    (Components|Activation|SetActive _array_element false false))
  (Components|Activation|SetActive CameraComponentToMakeActive true false)
  (Default|SetNewCamera (Variables|Default|GetCurrentInstigatingCharacter) self BlendTime BlendFunc BlendExp bLockOutgoing))

(fn GetComponentbyName
  (params (ComponentName :type String))
  (LocalVariables|SetComponentFoundLocal false)
  (for _array_element (Components|GetChildrenComponents (Variables|Default|GetDefaultSceneRoot) true)
    (if (Utilities|Enum|Equal(Enum) (Utilities|GetObjectName _array_element) ComponentName)
      (bind _asr_interaction (Utilities|Casting|CastToR_Interaction _array_element))
      (return _asr_interaction true)))
  (return 0 false))