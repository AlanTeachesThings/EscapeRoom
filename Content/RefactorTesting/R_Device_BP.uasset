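; R_Device_BP is an interactable device actor that relays highlight and interaction events to its R_Interaction components.
; It caches those components at BeginPlay, then loops over them to add or remove highlights and to signal the start of a parent interaction.
; After notifying them, it immediately tells the instigating character to end the interaction.
; Examine, press, directional control and back events are empty stubs.
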(event Custom|AddHighlights
  (for _array_element (Variables|Default|GetInteractionComponents)
    (Default|AddHighlight _array_element)))

(event Custom|RemoveHighlights
  (for _array_element (Variables|Default|GetInteractionComponents)
    (Default|RemoveHighlight _array_element)))

(event Custom|EndExamine
  (params (InstigatingCharacter :type BP%20First%20Person%20Character%20Object%20Reference)))

(event Custom|InteractStart
  (params (InstigatingCharacter :type BP%20First%20Person%20Character%20Object%20Reference)))

(event Custom|InteractDirectionalControl
  (params (ControlValues :type Vector%202D%20Structure) (InstigatingCharacter :type BP%20First%20Person%20Character%20Object%20Reference)))

(event Custom|InteractBack
  (params (InstigatingCharacter :type BP%20First%20Person%20Character%20Object%20Reference)))

(event Custom|InteractPressTick
  (params (InstigatingCharacter :type BP%20First%20Person%20Character%20Object%20Reference)))

(event Custom|InteractPressStart
  (params (InstigatingCharacter :type BP%20First%20Person%20Character%20Object%20Reference)))

(event Custom|OnBeginInteraction
  (params (InstigatingCharacter :type Escape%20Room%20Character%20Object%20Reference))
  (Utilities|FlowControl|Sequence
    (:then_0
      ;[0.15 0.15 0.15 0.5] Call Begin Parent Interaction on all Interaction Components
      (for _array_element (Variables|Default|GetInteractionComponents)
        (Default|OnBeginParentInteraction _array_element)))
    (:then_1
      ;[1 0 0 0.5] If nothing captures the player, then end interaction
      (Default|EndInteraction InstigatingCharacter))))

(event Custom|InteractPressEnd
  (params (InstigatingCharacter :type BP%20First%20Person%20Character%20Object%20Reference)))

(event Custom|Examine
  (params (InstigatingCharacter :type BP%20First%20Person%20Character%20Object%20Reference)))

(event EventBeginPlay
  (Variables|Default|SetInteractionComponents (Actor|GetComponentsByClass "/Game/RefactorTesting/R_Interaction.R_Interaction_C")))

(fn ConstructionScript)