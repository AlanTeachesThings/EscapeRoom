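; Escape-room slot interactable that accepts held items listed as unlocking or non-unlocking, or any item if it is a universal slot.
; Interacting with an accepted item hands any current key to the player, then a timeline lerps the new one onto ObjectSpot.
; Once placed, unlocking items send a value to targeted objects.
; Interacting empty-handed triggers the slotted key's own interaction to take it back.
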(event EventInteractStart
  (params (InstigatingCharacter :type BP%20First%20Person%20Character%20Object%20Reference))
  (bind _objectspot (Variables|Default|GetObjectSpot))
  (if (Utilities|IsValid (Variables|/Game/FirstPerson/Blueprints/BP_FirstPersonCharacter.BP_FirstPersonCharacter_C|GetCurrentHeldObject InstigatingCharacter))
    (Variables|Default|SetCurrentInstigatingCharacter InstigatingCharacter)
    (if (Math|Boolean|ORBoolean (>= (Utilities|Array|FindItem (Variables|SlotSetup|GetItemsNotForUnlock) (Variables|/Game/FirstPerson/Blueprints/BP_FirstPersonCharacter.BP_FirstPersonCharacter_C|GetCurrentHeldObject InstigatingCharacter)) 0) (>= (Utilities|Array|FindItem (Variables|SlotSetup|GetItemsForUnlock) (Variables|/Game/FirstPerson/Blueprints/BP_FirstPersonCharacter.BP_FirstPersonCharacter_C|GetCurrentHeldObject InstigatingCharacter)) 0) (Variables|SlotSetup|GetisUniversalSlot))
      ;[1 0 0 0.5] Swap Current Key Into Player's Hand!!!
      (Utilities|IsValid (Variables|Default|GetCurrentKey)
        (:Is%20Valid
          (Default|InteractStart (Variables|Default|GetCurrentKey) (Variables|Default|GetCurrentInstigatingCharacter)))
        (:Is%20Not%20Valid
          _))
      ;[0.15 0.15 0.15 0.5] Detach Key from Character and warp into place
      (Transformation|DetachFromActor (Variables|/Game/FirstPerson/Blueprints/BP_FirstPersonCharacter.BP_FirstPersonCharacter_C|GetCurrentHeldObject InstigatingCharacter) "KeepWorld" "KeepWorld" "KeepWorld")
      (Variables|Default|SetCurrentKey (Variables|/Game/FirstPerson/Blueprints/BP_FirstPersonCharacter.BP_FirstPersonCharacter_C|GetCurrentHeldObject InstigatingCharacter))
      (Variables|Default|SetKeyStartingLocation (Transformation|GetActorLocation (Variables|/Game/FirstPerson/Blueprints/BP_FirstPersonCharacter.BP_FirstPersonCharacter_C|GetCurrentHeldObject (Variables|Default|GetCurrentInstigatingCharacter))))
      (Variables|Default|SetKeyStartingRotation (Transformation|GetActorRotation (Variables|/Game/FirstPerson/Blueprints/BP_FirstPersonCharacter.BP_FirstPersonCharacter_C|GetCurrentHeldObject (Variables|Default|GetCurrentInstigatingCharacter))))
      (bind _lerpvalue (Timeline|ObjectLerpIntoPlace PlayFromStart)
        (:Update
          (Transformation|SetActorLocationAndRotation (Variables|Default|GetCurrentKey) (Math|Vector|Lerp(Vector) (Variables|Default|GetKeyStartingLocation) (Transformation|GetWorldLocation _objectspot) _lerpvalue) (Math|Rotator|Lerp(Rotator) (Variables|Default|GetKeyStartingRotation) (Transformation|GetWorldRotation _objectspot) _lerpvalue true)))
        (:Finished
          (Utilities|FlowControl|Sequence
            (:then_0
              (Variables|/Game/EscapeRoom/Interactions/PickUp/PickupBase_BP.PickupBase_BP_C|SetCurrentSlot (Variables|Default|GetCurrentKey) self))
            (:then_1
              (if (>= (Utilities|Array|FindItem (Variables|SlotSetup|GetItemsForUnlock) (Variables|Default|GetCurrentKey)) 0)
                (CallFunction|SendValuetoTargetedObjects (Variables|InteractSystem|GetValueToSendOnUnlock))))
            (:then_2
              (if (== (Variables|/Game/FirstPerson/Blueprints/BP_FirstPersonCharacter.BP_FirstPersonCharacter_C|GetCurrentHeldObject (Variables|Default|GetCurrentInstigatingCharacter)) (Variables|Default|GetCurrentKey))
                (Variables|/Game/FirstPerson/Blueprints/BP_FirstPersonCharacter.BP_FirstPersonCharacter_C|SetCurrentHeldObject (Variables|Default|GetCurrentInstigatingCharacter) 0))
              (Utilities|IsValid (Variables|Default|GetCurrentKey)
                (:Is%20Valid
                  (Collision|SetActorEnableCollision (Variables|Default|GetCurrentKey) true))
                (:Is%20Not%20Valid
                  _))
              (Default|EndInteraction (Variables|Default|GetCurrentInstigatingCharacter) :!label _label)))))
      (else
        (goto _label)))
    (else
      (Utilities|IsValid (Variables|Default|GetCurrentKey)
        (:Is%20Valid
          (Default|InteractStart (Variables|Default|GetCurrentKey) InstigatingCharacter)
          (Default|EndInteraction InstigatingCharacter))))))

(fn ConstructionScript
  (|CallParentFunction))