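; Examinable escape-room object that moves in front of the interacting character for inspection, then returns to its place.
; InteractStart saves the original transform, switches to the examine camera and timeline-lerps the actor to the character's offset ExamineSpot; its look-at rotation lerp has no Alpha wired.
; Directional input rotates the object locally, except during the return.
; InteractBack lerps position and rotation back, then ends the interaction.
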(event EventInteractStart
  (params (InstigatingCharacter :type BP%20First%20Person%20Character%20Object%20Reference))
  (CallFunction|RemoveHighlight)
  (Variables|Default|SetOriginalPosition (Transformation|GetActorLocation))
  (Variables|Default|SetOriginalRotation (Transformation|GetActorRotation))
  (bind _output_get (Variables|Default|SetInstigatingCharacter InstigatingCharacter))
  (Transformation|SetRelativeLocation (Variables|/Game/FirstPerson/Blueprints/BP_FirstPersonCharacter.BP_FirstPersonCharacter_C|GetExamineSpot _output_get) (Math|Vector|MakeVector (Variables|Default|GetExamineOffset) 0.0 0.0) false false)
  (Variables|/Game/FirstPerson/Blueprints/BP_FirstPersonCharacter.BP_FirstPersonCharacter_C|SetuseExamineCamera _output_get true)
  (bind _lerp (Timeline|LerpPositionIn PlayFromStart)
    (:Update
      (Transformation|SetActorLocation (Math|Vector|Lerp(Vector) (Variables|Default|GetOriginalPosition) (Transformation|GetWorldLocation (Variables|/Game/FirstPerson/Blueprints/BP_FirstPersonCharacter.BP_FirstPersonCharacter_C|GetExamineSpot (Variables|Default|GetInstigatingCharacter))) _lerp) false false)
      (Transformation|SetActorRotation (Math|Rotator|Lerp(Rotator) (Variables|Default|GetOriginalRotation) (Math|Rotator|FindLookatRotation (Variables|Default|GetOriginalPosition) (Transformation|GetWorldLocation (Variables|/Game/FirstPerson/Blueprints/BP_FirstPersonCharacter.BP_FirstPersonCharacter_C|GetExamineSpot (Variables|Default|GetInstigatingCharacter)))) 0.0 true)))))

(event EventInteractBack
  (params (InstigatingCharacter :type BP%20First%20Person%20Character%20Object%20Reference))
  (Variables|Default|SetTransitioning true)
  (Variables|/Game/FirstPerson/Blueprints/BP_FirstPersonCharacter.BP_FirstPersonCharacter_C|SetuseExamineCamera InstigatingCharacter false)
  (Variables|Default|SetEndRotation (Transformation|GetActorRotation))
  (bind _lerp (Timeline|LerpPositionOut PlayFromStart)
    (:Update
      (Transformation|SetActorLocation (Math|Vector|Lerp(Vector) (Transformation|GetWorldLocation (Variables|/Game/FirstPerson/Blueprints/BP_FirstPersonCharacter.BP_FirstPersonCharacter_C|GetExamineSpot (Variables|Default|GetInstigatingCharacter))) (Variables|Default|GetOriginalPosition) _lerp) false false)
      (Transformation|SetActorRotation (Math|Rotator|Lerp(Rotator) (Variables|Default|GetEndRotation) (Variables|Default|GetOriginalRotation) _lerp true)))
    (:Finished
      (Default|EndInteraction (Variables|Default|GetInstigatingCharacter))
      (Variables|Default|SetTransitioning false))))

(event EventInteractDirectionalControl
  (params (ControlValues :type Vector%202D%20Structure) (InstigatingCharacter :type BP%20First%20Person%20Character%20Object%20Reference))
  (bind _rotationspeed (Variables|Default|GetRotationSpeed))
  (bind _returnvalue (* ControlValues _rotationspeed))
  (if (not (Variables|Default|GetTransitioning))
    (Transformation|AddActorLocalRotation (Math|Rotator|MakeRotator 0.0 (.y _returnvalue) (.x _returnvalue)) false false)))

(fn ConstructionScript
  (|CallParentFunction))