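; Dial_BP is an escape room interactable dial that the player rotates in discrete steps to feed a value to other objects.
; Directional input past a threshold on the horizontal or vertical axis sets the turn direction and plays a timeline that rotates the mesh one step, ignoring input mid-turn.
; When the turn finishes, it wraps the position within the step count and sends it to targeted objects.
; Back ends the interaction.
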(event EventBeginPlay
  (|CallParentFunction)
  (Variables|Default|SetCurrentPosition (Variables|Default|GetStartingPosition)))

(event EventInteractStart
  (params (InstigatingCharacter :type BP%20First%20Person%20Character%20Object%20Reference))
  (CallFunction|RemoveHighlight))

(event EventInteractDirectionalControl
  (params (ControlValues :type Vector%202D%20Structure) (InstigatingCharacter :type BP%20First%20Person%20Character%20Object%20Reference))
  (bind _horizontal (Variables|Default|GetHorizontal))
  (bind _rotationsteps (Variables|Default|GetRotationSteps))
  (bind _returnvalue (Math|Float|SelectFloat (.x ControlValues) (.y ControlValues) _horizontal))
  (if (not (Variables|Default|GetisRotating))
    (Variables|Default|SetLastRelativeRotation (Variables|/Script/Engine.SceneComponent|GetRelativeRotation (Variables|Default|GetStaticMesh)))
    (if (> _returnvalue 0.9)
      (Variables|Default|SetDirectionMultiplier 1.0)
      (bind _additionalrelativerotationalpha (Timeline|RotationTimeline PlayFromStart)
        (:Update
          (Transformation|SetRelativeRotation (Variables|Default|GetStaticMesh) (Math|Rotator|CombineRotators (Variables|Default|GetLastRelativeRotation) (Math|Rotator|SelectRotator (Math|Rotator|MakeRotator (.roll (Variables|Default|GetLastRelativeRotation)) (.pitch (Variables|Default|GetLastRelativeRotation)) (+ (.pitch (Variables|Default|GetLastRelativeRotation)) (* _additionalrelativerotationalpha (/ 3.6e+02 (Math|Conversions|ToFloat(Integer) (Variables|Default|GetRotationSteps))) (Variables|Default|GetDirectionMultiplier)))) (Math|Rotator|MakeRotator (.roll (Variables|Default|GetLastRelativeRotation)) (+ (* _additionalrelativerotationalpha (/ 3.6e+02 (Math|Conversions|ToFloat(Integer) (Variables|Default|GetRotationSteps))) (Variables|Default|GetDirectionMultiplier)) (.yaw (Variables|Default|GetLastRelativeRotation))) (.yaw (Variables|Default|GetLastRelativeRotation))) (Variables|Default|GetHorizontal))) false false)
          (Variables|Default|SetisRotating true))
        (:Finished
          (Variables|Default|SetisRotating false)
          (bind _output_get (Variables|Default|SetCurrentPosition (Math|Integer|SelectInt (- _rotationsteps 1) (Math|Integer|SelectInt 0 (+ (Variables|Default|GetCurrentPosition) (Variables|Default|GetDirectionMultiplier)) (== (+ (Variables|Default|GetCurrentPosition) (Variables|Default|GetDirectionMultiplier)) _rotationsteps)) (< (Math|Integer|SelectInt 0 (+ (Variables|Default|GetCurrentPosition) (Variables|Default|GetDirectionMultiplier)) (== (+ (Variables|Default|GetCurrentPosition) (Variables|Default|GetDirectionMultiplier)) _rotationsteps)) 0))))
          (CallFunction|SendValuetoTargetedObjects _output_get)))
      (elif (< _returnvalue -0.9)
        (Variables|Default|SetDirectionMultiplier -1.0)
        (Timeline|RotationTimeline PlayFromStart)))))

(event EventInteractBack
  (params (InstigatingCharacter :type BP%20First%20Person%20Character%20Object%20Reference))
  (Default|EndInteraction InstigatingCharacter))

(fn ConstructionScript
  (|CallParentFunction))