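; Base Blueprint for escape room interactables, with mostly empty examine and interact events and a default interaction style.
; Highlighting attaches Niagara systems to every static and skeletal mesh, with paired DoOnce gates so add and remove alternate cleanly.
; Values are relayed to targeted objects, which gain the parent actor when this is a child actor.
; It tracks the last instigating character and can end their interaction on a reported unlock.
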(event Custom|AddHighlight
  (Utilities|FlowControl|DoOnce false
    (:Completed
      (Utilities|FlowControl|Sequence
        (:then_0
          (for _array_element (Actor|GetComponentsByClass "/Script/Engine.StaticMeshComponent")
            (bind _returnvalue (Niagara|SpawnSystemAttached "/Game/EscapeRoom/Interactions/VFX/HighlightSystemStatic_NS.HighlightSystemStatic_NS" _array_element "None" "0, 0, 0" "0, 0, 0" "KeepRelativeOffset" false))
            (Utilities|Array|Add (Variables|Default|GetHighlightSystemComponents) _returnvalue)))
        (:then_1
          (for _array_element_2 (Actor|GetComponentsByClass "/Script/Engine.SkeletalMeshComponent")
            (bind _returnvalue_2 (Niagara|SpawnSystemAttached "/Game/EscapeRoom/Interactions/VFX/HighlightSystemSkeletal_NS.HighlightSystemSkeletal_NS" _array_element_2 "None" "0, 0, 0" "0, 0, 0" "KeepRelativeOffset" false))
            (Utilities|Array|Add (Variables|Default|GetHighlightSystemComponents) _returnvalue_2)))
        (:then_2
          (Utilities|FlowControl|DoOnce false) ; enters at Reset
        )))))

(event Custom|RemoveHighlight
  (Utilities|FlowControl|DoOnce false
    (:Completed
      (Utilities|FlowControl|Sequence
        (:then_0
          (for _array_element (Variables|Default|GetHighlightSystemComponents)
            (Utilities|IsValid _array_element
              (:Is%20Valid
                (Components|DestroyComponent _array_element))))
          (Utilities|Array|Clear (Variables|Default|GetHighlightSystemComponents)))
        (:then_1
          (Utilities|FlowControl|DoOnce false) ; enters at Reset
        )))))

(event Custom|SendValueToTargetedObjects
  (params (ValueToSend :type Integer))
  (bind _self self)
  (for _array_element (Variables|InteractSystem|GetTargetedObjects)
    (Class|ObjectInterface|ReceiveValue(Message) _array_element _self ValueToSend)
    (Development|PrintString (Utilities|String|Append (Utilities|GetDisplayName _self) " sent " (Utilities|String|ToString(Integer) ValueToSend) " to " (Utilities|GetDisplayName _array_element)))))

(event Custom|EndExamine
  (params (InstigatingCharacter :type BP%20First%20Person%20Character%20Object%20Reference)))

(event Custom|InteractStart
  (params (InstigatingCharacter :type BP%20First%20Person%20Character%20Object%20Reference))
  (Variables|Default|SetLastInstigatingCharacter InstigatingCharacter))

(event Custom|InteractDirectionalControl
  (params (ControlValues :type Vector%202D%20Structure) (InstigatingCharacter :type BP%20First%20Person%20Character%20Object%20Reference)))

(event Custom|InteractBack
  (params (InstigatingCharacter :type BP%20First%20Person%20Character%20Object%20Reference))
  (Variables|Default|GetisBeingExamined
    (:then
      (CallFunction|EndExamine InstigatingCharacter))
    (:else)))

(event Custom|InteractPressTick
  (params (InstigatingCharacter :type BP%20First%20Person%20Character%20Object%20Reference)))

(event Custom|InteractPressStart
  (params (InstigatingCharacter :type BP%20First%20Person%20Character%20Object%20Reference)))

(event Custom|ReportUnlockSuccesful
  (params (ReportingActor :type Actor%20Object%20Reference))
  (if (Variables|InteractSystem|GetEndInteractionOnUnlock)
    (Default|EndInteraction (Variables|Default|GetLastInstigatingCharacter))))

(event Custom|InteractPressEnd
  (params (InstigatingCharacter :type BP%20First%20Person%20Character%20Object%20Reference)))

(event Custom|Examine
  (params (InstigatingCharacter :type BP%20First%20Person%20Character%20Object%20Reference)))

(event EventBeginPlay
  (if (Class|Actor|IsChildActor)
    (Utilities|Array|Add (Variables|InteractSystem|GetTargetedObjects) (Actor|GetAttachParentActor))))

(fn ConstructionScript)

(fn GetInteractionStyle
  (params (InstigatingCharacter :type BP%20First%20Person%20Character%20Object%20Reference))
  (return (Variables|InteractSystem|GetDefaultInteractionStyle)))