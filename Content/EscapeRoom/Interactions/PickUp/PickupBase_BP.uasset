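; Base pickup Blueprint for the escape room that lets a character pick up the object and hold it.
; On interaction it clears its highlight, disables collision and uses a timeline to lerp position and rotation to the character's PickUpSpot.
; When the lerp finishes it attaches to that spot, becomes the character's held object, clears itself from any key slot and ends the interaction.
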(event EventInteractStart
  (params (InstigatingCharacter :type BP%20First%20Person%20Character%20Object%20Reference))
  (bind _currentslot (Variables|Default|GetCurrentSlot))
  (Variables|Default|SetCurrentInstigatingCharacter InstigatingCharacter)
  (CallFunction|RemoveHighlight)
  (Variables|Default|SetStartingLocation (Transformation|GetActorLocation))
  (Variables|Default|SetStartingRotation (Transformation|GetActorRotation))
  (Collision|SetActorEnableCollision false)
  (bind _lerpalpha (Timeline|PositionAndRotationLerp PlayFromStart)
    (:Update
      (Transformation|SetActorLocationAndRotation (Math|Vector|Lerp(Vector) (Variables|Default|GetStartingLocation) (Transformation|GetWorldLocation (Variables|/Game/FirstPerson/Blueprints/BP_FirstPersonCharacter.BP_FirstPersonCharacter_C|GetPickUpSpot (Variables|Default|GetCurrentInstigatingCharacter))) _lerpalpha) (Math|Rotator|Lerp(Rotator) (Variables|Default|GetStartingRotation) (Transformation|GetWorldRotation (Variables|/Game/FirstPerson/Blueprints/BP_FirstPersonCharacter.BP_FirstPersonCharacter_C|GetPickUpSpot (Variables|Default|GetCurrentInstigatingCharacter))) _lerpalpha true)))
    (:Finished
      (Variables|/Game/FirstPerson/Blueprints/BP_FirstPersonCharacter.BP_FirstPersonCharacter_C|SetCurrentHeldObject (Variables|Default|GetCurrentInstigatingCharacter) self)
      (Transformation|AttachComponentToComponent (Variables|/Game/FirstPerson/Blueprints/BP_FirstPersonCharacter.BP_FirstPersonCharacter_C|GetPickUpSpot (Variables|Default|GetCurrentInstigatingCharacter)) "None" "KeepWorld" "KeepWorld" "KeepWorld" true)
      (Utilities|IsValid _currentslot
        (:Is%20Valid
          (Variables|/Game/EscapeRoom/Interactions/Slot/Slot_BP.Slot_BP_C|SetCurrentKey _currentslot 0))
        (:Is%20Not%20Valid
          _))
      (Default|EndInteraction (Variables|Default|GetCurrentInstigatingCharacter)))))

(fn ConstructionScript
  (|CallParentFunction))