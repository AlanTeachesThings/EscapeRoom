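; Interactable furniture helper for the escape room that moves and rotates a static mesh between its rest pose and a target pose.
; When unlocked, each interaction alternates playing a float Curve forward or backward from its endpoint, then immediately ends the interaction.
; Tick drives the lerp while ElapsedTime is within the curve's range, and prints a warning without a curve.
; SetMesh assigns the mesh and snaps it to either pose.
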(event EventTick
  (params (DeltaSeconds :type Float%20%28single-precision%29))
  (bind _curve (Variables|Default|GetCurve))
  (bind _staticmesh (Variables|Default|GetStaticMesh))
  (bind (_mintime _maxtime) (Math|Curves|GetTimeRange _curve))
  (Utilities|IsValid _curve
    (:Is%20Valid
      (if (and (>= (Variables|Default|GetElapsedTime) _mintime) (<= (Variables|Default|GetElapsedTime) _maxtime))
        (bind _output_get (Variables|Default|SetElapsedTime (+ (Variables|Default|GetElapsedTime) (* (Variables|Default|GetTimeDirection) DeltaSeconds))))
        (Transformation|SetRelativeLocation _staticmesh (Math|Vector|Lerp(Vector) "0, 0, 0" (Variables|Default|GetTargetLocation) (Math|Curves|GetFloatValue (Variables|Default|GetCurve) _output_get)) false false)
        (Transformation|SetRelativeRotation _staticmesh (Math|Rotator|Lerp(Rotator) "0, 0, 0" (Variables|Default|GetTargetRotation) (Math|Curves|GetFloatValue (Variables|Default|GetCurve) _output_get)) false false)))
    (:Is%20Not%20Valid
      (Development|PrintString (Utilities|String|Append (Utilities|GetDisplayName self) " has a missing curve!")))))

(event EventBeginPlay
  (bind _staticmesh (Variables|Default|GetStaticMesh))
  (|CallParentFunction)
  (Utilities|FlowControl|DelayUntilNextTick)
  (Transformation|SetRelativeLocation _staticmesh "0, 0, 0" false false)
  (Transformation|SetRelativeRotation _staticmesh "0, 0, 0" false false)
  (Variables|Default|SetElapsedTime 99999.0))

(event EventInteractStart
  (params (InstigatingCharacter :type BP%20First%20Person%20Character%20Object%20Reference))
  (bind _curve (Variables|Default|GetCurve))
  (bind (_mintime _maxtime) (Math|Curves|GetTimeRange _curve))
  (|CallParentFunction InstigatingCharacter)
  (if (Variables|Default|GetisLocked)
    _
    (else
      (Utilities|FlowControl|FlipFlop
        (:A
          (Variables|Default|SetTimeDirection 1.0)
          (Variables|Default|SetElapsedTime _mintime))
        (:B
          (Variables|Default|SetTimeDirection -1.0)
          (Variables|Default|SetElapsedTime _maxtime)))))
  (Default|EndInteraction InstigatingCharacter))

(fn ConstructionScript
  (|CallParentFunction))

(fn SetMesh
  (params (SetToTarget :type Boolean))
  (bind _staticmesh (Variables|Default|GetStaticMesh))
  (Components|StaticMesh|SetStaticMesh _staticmesh (Variables|Default|GetMeshToMove))
  (Transformation|SetRelativeLocation _staticmesh (Math|Vector|SelectVector (Variables|Default|GetTargetLocation) "0, 0, 0" SetToTarget) false false)
  (Transformation|SetRelativeRotation _staticmesh (Math|Rotator|SelectRotator (Variables|Default|GetTargetRotation) "0, 0, 0" SetToTarget) false false))