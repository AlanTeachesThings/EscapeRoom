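; Sliding puzzle tile for the escape room that moves itself one grid step into the first open space when interacted with.
; It tries right, left, down, then up in local X/Z, requiring each step to stay within limits and pass a box trace.
; The block moves with a swept relative offset.
; InteractPressStart drives it as a child actor, InteractStart otherwise, both sharing the same logic.
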(event EventInteractPressStart
  (params (InstigatingCharacter :type BP%20First%20Person%20Character%20Object%20Reference))
  (bind _gridsnapsize (Variables|Default|GetGridSnapSize))
  (bind _slidingblock (Variables|Default|GetSlidingBlock))
  (bind _slidingblock_2 (Variables|Default|GetSlidingBlock))
  (bind _slidingblock_3 (Variables|Default|GetSlidingBlock))
  (bind _slidingblock_4 (Variables|Default|GetSlidingBlock))
  (bind _slidingblock_5 (Variables|Default|GetSlidingBlock))
  (bind _slidingblock_6 (Variables|Default|GetSlidingBlock))
  (bind _gridsnapsize_2 (Variables|Default|GetGridSnapSize))
  (bind _slidingblock_7 (Variables|Default|GetSlidingBlock))
  (bind _gridsnapsize_3 (Variables|Default|GetGridSnapSize))
  (bind _slidingblock_8 (Variables|Default|GetSlidingBlock))
  (bind _gridsnapsize_4 (Variables|Default|GetGridSnapSize))
  (bind _returnvalue (Transformation|GetWorldRotation _slidingblock_7))
  (bind _returnvalue_2 (Transformation|GetWorldRotation _slidingblock_8))
  (bind _returnvalue_3 (Transformation|GetWorldRotation _slidingblock))
  (bind _returnvalue_4 (Transformation|GetWorldRotation _slidingblock_2))
  (bind _returnvalue_5 (Math|Vector|MakeVector _gridsnapsize_2 0.0 0.0))
  (bind _returnvalue_6 (Math|Vector|MakeVector 0.0 0.0 _gridsnapsize))
  (bind _returnvalue_7 (Transformation|GetWorldLocation _slidingblock_3))
  (bind _returnvalue_8 (Transformation|GetWorldLocation _slidingblock_4))
  (bind _returnvalue_9 (Transformation|GetWorldLocation _slidingblock_5))
  (bind _returnvalue_10 (Transformation|GetWorldLocation _slidingblock_6))
  (bind _returnvalue_11 (* _gridsnapsize_3 -1.0))
  (bind _returnvalue_12 (* _gridsnapsize_4 -1.0))
  (bind _returnvalue_13 (Math|Vector|RotateVector _returnvalue_5 _returnvalue))
  (bind _returnvalue_14 (Math|Vector|MakeVector _returnvalue_11 0.0 0.0))
  (bind _returnvalue_15 (Math|Vector|MakeVector 0.0 0.0 _returnvalue_12))
  (bind _returnvalue_16 (Math|Vector|RotateVector _returnvalue_6 _returnvalue_3))
  (bind _returnvalue_17 (Math|Vector|RotateVector _returnvalue_14 _returnvalue_2))
  (bind _returnvalue_18 (Math|Vector|RotateVector _returnvalue_15 _returnvalue_4))
  (bind _returnvalue_19 (+ _returnvalue_7 _returnvalue_16))
  (bind _returnvalue_20 (+ _returnvalue_8 _returnvalue_13))
  (bind _returnvalue_21 (+ _returnvalue_9 _returnvalue_17))
  (bind _returnvalue_22 (+ _returnvalue_10 _returnvalue_18))
  (if (Class|Actor|IsChildActor)
    (Variables|Default|SetFoundMoveDirection false)
    (if (not (Variables|Default|GetFoundMoveDirection))
      (if (CallFunction|IsStepWithinLimits _returnvalue_5)
        (bind _returnvalue_23 (Collision|BoxTraceByChannel _returnvalue_20 _returnvalue_20 (.Max (Components|StaticMesh|GetLocalBounds _slidingblock_7)) _returnvalue "TraceTypeQuery1" false 0 "None"))
        (if _returnvalue_23
          (if (not (Variables|Default|GetFoundMoveDirection)) :!label _label
            (if (CallFunction|IsStepWithinLimits _returnvalue_14)
              (bind _returnvalue_24 (Collision|BoxTraceByChannel _returnvalue_21 _returnvalue_21 (.Max (Components|StaticMesh|GetLocalBounds _slidingblock_8)) _returnvalue_2 "TraceTypeQuery1" false 0 "None"))
              (if _returnvalue_24
                (if (not (Variables|Default|GetFoundMoveDirection)) :!label _label_2
                  (if (CallFunction|IsStepWithinLimits _returnvalue_15)
                    (bind _returnvalue_25 (Collision|BoxTraceByChannel _returnvalue_22 _returnvalue_22 (.Max (Components|StaticMesh|GetLocalBounds _slidingblock_2)) _returnvalue_4 "TraceTypeQuery1" false 0 "None"))
                    (if _returnvalue_25
                      (if (CallFunction|IsStepWithinLimits _returnvalue_6) :!label _label_3
                        (bind _returnvalue_26 (Collision|BoxTraceByChannel _returnvalue_19 _returnvalue_19 (.Max (Components|StaticMesh|GetLocalBounds _slidingblock)) _returnvalue_3 "TraceTypeQuery1" false 0 "None"))
                        (if _returnvalue_26
                          (Development|PrintString "Up Move Blocked!")
                          (else
                            (Variables|Default|SetFoundMoveDirection true)
                            (Transformation|AddRelativeLocation (Variables|Default|GetSlidingBlock) _returnvalue_6 true false)))
                        (else
                          (Development|PrintString "Up Move Outside Limits!")))
                      (else
                        (Variables|Default|SetFoundMoveDirection true)
                        (Transformation|AddRelativeLocation (Variables|Default|GetSlidingBlock) _returnvalue_15 true false)))
                    (else
                      (Development|PrintString "Down Move Outside Limits")
                      (goto _label_3))))
                (else
                  (Variables|Default|SetFoundMoveDirection true)
                  (Transformation|AddRelativeLocation (Variables|Default|GetSlidingBlock) _returnvalue_14 true false)))
              (else
                (Development|PrintString "Left Move Outside Limits")
                (goto _label_2))))
          (else
            (Variables|Default|SetFoundMoveDirection true)
            (Transformation|AddRelativeLocation (Variables|Default|GetSlidingBlock) _returnvalue_5 true false)))
        (else
          (Development|PrintString "Right Move Outside Limits ")
          (goto _label))))))

(event EventInteractStart
  (params (InstigatingCharacter :type BP%20First%20Person%20Character%20Object%20Reference))
  (bind _gridsnapsize (Variables|Default|GetGridSnapSize))
  (bind _slidingblock (Variables|Default|GetSlidingBlock))
  (bind _slidingblock_2 (Variables|Default|GetSlidingBlock))
  (bind _slidingblock_3 (Variables|Default|GetSlidingBlock))
  (bind _slidingblock_4 (Variables|Default|GetSlidingBlock))
  (bind _slidingblock_5 (Variables|Default|GetSlidingBlock))
  (bind _slidingblock_6 (Variables|Default|GetSlidingBlock))
  (bind _gridsnapsize_2 (Variables|Default|GetGridSnapSize))
  (bind _slidingblock_7 (Variables|Default|GetSlidingBlock))
  (bind _gridsnapsize_3 (Variables|Default|GetGridSnapSize))
  (bind _slidingblock_8 (Variables|Default|GetSlidingBlock))
  (bind _gridsnapsize_4 (Variables|Default|GetGridSnapSize))
  (bind _returnvalue (Transformation|GetWorldRotation _slidingblock_7))
  (bind _returnvalue_2 (Transformation|GetWorldRotation _slidingblock_8))
  (bind _returnvalue_3 (Transformation|GetWorldRotation _slidingblock))
  (bind _returnvalue_4 (Transformation|GetWorldRotation _slidingblock_2))
  (bind _returnvalue_5 (Math|Vector|MakeVector _gridsnapsize_2 0.0 0.0))
  (bind _returnvalue_6 (Math|Vector|MakeVector 0.0 0.0 _gridsnapsize))
  (bind _returnvalue_7 (Transformation|GetWorldLocation _slidingblock_3))
  (bind _returnvalue_8 (Transformation|GetWorldLocation _slidingblock_4))
  (bind _returnvalue_9 (Transformation|GetWorldLocation _slidingblock_5))
  (bind _returnvalue_10 (Transformation|GetWorldLocation _slidingblock_6))
  (bind _returnvalue_11 (* _gridsnapsize_3 -1.0))
  (bind _returnvalue_12 (* _gridsnapsize_4 -1.0))
  (bind _returnvalue_13 (Math|Vector|RotateVector _returnvalue_5 _returnvalue))
  (bind _returnvalue_14 (Math|Vector|MakeVector _returnvalue_11 0.0 0.0))
  (bind _returnvalue_15 (Math|Vector|MakeVector 0.0 0.0 _returnvalue_12))
  (bind _returnvalue_16 (Math|Vector|RotateVector _returnvalue_6 _returnvalue_3))
  (bind _returnvalue_17 (Math|Vector|RotateVector _returnvalue_14 _returnvalue_2))
  (bind _returnvalue_18 (Math|Vector|RotateVector _returnvalue_15 _returnvalue_4))
  (bind _returnvalue_19 (+ _returnvalue_7 _returnvalue_16))
  (bind _returnvalue_20 (+ _returnvalue_8 _returnvalue_13))
  (bind _returnvalue_21 (+ _returnvalue_9 _returnvalue_17))
  (bind _returnvalue_22 (+ _returnvalue_10 _returnvalue_18))
  (if (not (Class|Actor|IsChildActor))
    (Variables|Default|SetFoundMoveDirection false)
    (if (not (Variables|Default|GetFoundMoveDirection))
      (if (CallFunction|IsStepWithinLimits _returnvalue_5)
        (bind _returnvalue_23 (Collision|BoxTraceByChannel _returnvalue_20 _returnvalue_20 (.Max (Components|StaticMesh|GetLocalBounds _slidingblock_7)) _returnvalue "TraceTypeQuery1" false 0 "None"))
        (if _returnvalue_23
          (if (not (Variables|Default|GetFoundMoveDirection)) :!label _label
            (if (CallFunction|IsStepWithinLimits _returnvalue_14)
              (bind _returnvalue_24 (Collision|BoxTraceByChannel _returnvalue_21 _returnvalue_21 (.Max (Components|StaticMesh|GetLocalBounds _slidingblock_8)) _returnvalue_2 "TraceTypeQuery1" false 0 "None"))
              (if _returnvalue_24
                (if (not (Variables|Default|GetFoundMoveDirection)) :!label _label_2
                  (if (CallFunction|IsStepWithinLimits _returnvalue_15)
                    (bind _returnvalue_25 (Collision|BoxTraceByChannel _returnvalue_22 _returnvalue_22 (.Max (Components|StaticMesh|GetLocalBounds _slidingblock_2)) _returnvalue_4 "TraceTypeQuery1" false 0 "None"))
                    (if _returnvalue_25
                      (if (CallFunction|IsStepWithinLimits _returnvalue_6) :!label _label_3
                        (bind _returnvalue_26 (Collision|BoxTraceByChannel _returnvalue_19 _returnvalue_19 (.Max (Components|StaticMesh|GetLocalBounds _slidingblock)) _returnvalue_3 "TraceTypeQuery1" false 0 "None"))
                        (if _returnvalue_26
                          (Development|PrintString "Up Move Blocked!")
                          (else
                            (Variables|Default|SetFoundMoveDirection true)
                            (Transformation|AddRelativeLocation (Variables|Default|GetSlidingBlock) _returnvalue_6 true false)))
                        (else
                          (Development|PrintString "Up Move Outside Limits!")))
                      (else
                        (Variables|Default|SetFoundMoveDirection true)
                        (Transformation|AddRelativeLocation (Variables|Default|GetSlidingBlock) _returnvalue_15 true false)))
                    (else
                      (Development|PrintString "Down Move Outside Limits")
                      (goto _label_3))))
                (else
                  (Variables|Default|SetFoundMoveDirection true)
                  (Transformation|AddRelativeLocation (Variables|Default|GetSlidingBlock) _returnvalue_14 true false)))
              (else
                (Development|PrintString "Left Move Outside Limits")
                (goto _label_2))))
          (else
            (Variables|Default|SetFoundMoveDirection true)
            (Transformation|AddRelativeLocation (Variables|Default|GetSlidingBlock) _returnvalue_5 true false)))
        (else
          (Development|PrintString "Right Move Outside Limits ")
          (goto _label))))))

(fn ConstructionScript
  (|CallParentFunction))

(fn IsStepWithinLimits
  (params (RelativeLocationToTest :type Vector))
  (bind _slidingblock (Variables|Default|GetSlidingBlock))
  (bind _relativelocation (Variables|/Script/Engine.SceneComponent|GetRelativeLocation _slidingblock))
  (bind _returnvalue (+ (.x _relativelocation) (.x RelativeLocationToTest)))
  (bind _returnvalue_2 (+ (.z _relativelocation) (.z RelativeLocationToTest)))
  (return (and (and (<= _returnvalue (.x (Variables|Default|GetRightLimit))) (>= _returnvalue (.x (Variables|Default|GetLeftLimit)))) (and (<= _returnvalue_2 (.z (Variables|Default|GetUpperLimit))) (>= _returnvalue_2 (.z (Variables|Default|GetLowerLimit)))))))