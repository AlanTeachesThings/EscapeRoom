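; Escape room sliding tile interactable that the player drags by mouse or directional input to solve a lock.
; Movement is swept and clamped to X/Z limits; on release the block snaps to a grid and sends an unlock value to targeted objects if it sits at the target position.
; The construction script flattens limits to single axes, places a debug target marker and offsets a dynamic material to show one section of a divided texture.
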(event EventInteractStart
  (params (InstigatingCharacter :type BP%20First%20Person%20Character%20Object%20Reference))
  (Variables|Default|SetLastInstigatingCharacter InstigatingCharacter)
  (if (not (Class|Actor|IsChildActor))
    (Default|HideReticle (Variables|Default|GetLastInstigatingCharacter))
    (Variables|Default|SetcanSlide true)))

(event EventInteractPressStart
  (params (InstigatingCharacter :type BP%20First%20Person%20Character%20Object%20Reference))
  (Variables|Default|SetLastInstigatingCharacter InstigatingCharacter)
  (Variables|Default|SetcanSlide true))

(event EventInteractPressEnd
  (params (InstigatingCharacter :type BP%20First%20Person%20Character%20Object%20Reference))
  (bind _slidingblock (Variables|Default|GetSlidingBlock))
  (bind _gridsnapsize (Variables|Default|GetGridSnapSize))
  (bind _gridsnapsize_2 (Variables|Default|GetGridSnapSize))
  (bind _slidingblock_2 (Variables|Default|GetSlidingBlock))
  (bind _targetposition (Variables|InteractSystem|GetTargetPosition))
  (bind _relativelocation (Variables|/Script/Engine.SceneComponent|GetRelativeLocation _slidingblock))
  (bind _relativelocation_2 (Variables|/Script/Engine.SceneComponent|GetRelativeLocation _slidingblock_2))
  (Utilities|FlowControl|Sequence
    (:then_0
      (Variables|Default|SetcanSlide false))
    (:then_1
      ;[1 1 1] Snap to Grid
      (Transformation|SetRelativeLocation _slidingblock (Math|Vector|MakeVector (* (Math|Float|Round (/ (.x _relativelocation) _gridsnapsize)) _gridsnapsize_2) (.y _relativelocation) (* (Math|Float|Round (/ (.z _relativelocation) _gridsnapsize)) _gridsnapsize_2)) true false))
    (:then_2
      ;[1 1 1] ResolveLock
      (if (and (== (.x _targetposition) (.x _relativelocation_2)) (== (.z _relativelocation_2) (.y _targetposition)))
        (CallFunction|SendValuetoTargetedObjects (Variables|InteractSystem|GetValueToSendOnUnlock))))
    (:then_3
      ;[0.15 0.15 0.15 0.5] End Interaction
      (CallFunction|RemoveHighlight)
      (if (not (Class|Actor|IsChildActor))
        (Default|ShowReticle InstigatingCharacter)
        (Default|EndInteraction InstigatingCharacter)
        (Variables|Default|SetLastInstigatingCharacter 0)))))

(event EventInteractDirectionalControl
  (params (ControlValues :type Vector%202D%20Structure) (InstigatingCharacter :type BP%20First%20Person%20Character%20Object%20Reference))
  (bind _slidingblock (Variables|Default|GetSlidingBlock))
  (bind _dragspeed (Variables|Default|GetDragSpeed))
  (bind _relativelocation (Variables|/Script/Engine.SceneComponent|GetRelativeLocation _slidingblock))
  ;[0.15 0.15 0.15 0.5] Move with Mouse Control or Directional Input
  (Variables|Default|GetlastInputMouse
    (:then)
    (:else
      (Variables|Default|SetXInput (.x ControlValues))
      (Variables|Default|SetYInput (.y ControlValues))
      (Transformation|SetRelativeLocation _slidingblock (Math|Vector|MakeVector (Math|Float|Clamp(Float) (+ (.x _relativelocation) (* (Variables|Default|GetXInput) _dragspeed)) (.x (Variables|Default|GetLeftLimit)) (.x (Variables|Default|GetRightLimit))) (.y _relativelocation) (Math|Float|Clamp(Float) (+ (.z _relativelocation) (* _dragspeed (Variables|Default|GetYInput))) (.z (Variables|Default|GetLowerLimit)) (.z (Variables|Default|GetUpperLimit)))) true false))))

(event EventMouseInput
  (params (MouseMovement :type Vector :default "0, 0, 0") (InstigatingCharacter :type BP%20First%20Person%20Character%20Object%20Reference))
  (bind (_x _y) (Math|Vector|BreakVector MouseMovement))
  (bind _slidingblock (Variables|Default|GetSlidingBlock))
  (bind _dragspeed (Variables|Default|GetDragSpeed))
  (bind _relativelocation (Variables|/Script/Engine.SceneComponent|GetRelativeLocation _slidingblock))
  ;[0.15 0.15 0.15 0.5] Move with Mouse Control or Directional Input
  (if (Variables|Default|GetcanSlide)
    (Variables|Default|SetlastInputMouse (> (Math|Vector|VectorLength MouseMovement) 0.0))
    (Variables|Default|SetXInput _x)
    (Variables|Default|SetYInput _y)
    (Transformation|SetRelativeLocation _slidingblock (Math|Vector|MakeVector (Math|Float|Clamp(Float) (+ (.x _relativelocation) (* (Variables|Default|GetXInput) _dragspeed)) (.x (Variables|Default|GetLeftLimit)) (.x (Variables|Default|GetRightLimit))) (.y _relativelocation) (Math|Float|Clamp(Float) (+ (.z _relativelocation) (* _dragspeed (Variables|Default|GetYInput))) (.z (Variables|Default|GetLowerLimit)) (.z (Variables|Default|GetUpperLimit)))) true false)))

(fn ConstructionScript
  (bind _texturedivisions (Variables|Default|GetTextureDivisions))
  (bind _textureoffset (Variables|Default|GetTextureOffset))
  (bind _targetposition (Variables|InteractSystem|GetTargetPosition))
  (bind _returnvalue (/ 1.0 _texturedivisions))
  (bind _returnvalue_2 (* _returnvalue _textureoffset))
  (|CallParentFunction)
  (Utilities|FlowControl|Sequence
    (:then_0
      (Variables|Default|SetUpperLimit (Math|Vector|MakeVector 0.0 0.0 (.z (Variables|Default|GetUpperLimit))))
      (Variables|Default|SetLowerLimit (Math|Vector|MakeVector 0.0 0.0 (.z (Variables|Default|GetLowerLimit))))
      (Variables|Default|SetLeftLimit (Math|Vector|MakeVector (.x (Variables|Default|GetLeftLimit)) 0.0 0.0))
      (Variables|Default|SetRightLimit (Math|Vector|MakeVector (.x (Variables|Default|GetRightLimit)) 0.0 0.0)))
    (:then_1
      (Transformation|SetRelativeLocation (Variables|Default|GetDebugTargetMarker) (Math|Vector|MakeVector (.x _targetposition) 0.0 (.y _targetposition)) false false))
    (:then_2
      (bind _returnvalue_3 (Rendering|Material|CreateDynamicMaterialInstance "/Game/EscapeRoom/Interactions/SlidingTile/Mat/Tile_M.Tile_M" "None" "None" :!class /Script/Engine.KismetMaterialLibrary))
      (bind _output_get (Variables|Default|SetTileMaterialInstance _returnvalue_3))
      (Rendering|Material|SetMaterial (Variables|Default|GetSlidingBlock) 0 _output_get)
      (Rendering|Material|SetScalarParameterValue (Variables|Default|GetTileMaterialInstance) "XOffset" (.x _returnvalue_2) :!class /Script/Engine.MaterialInstanceDynamic)
      (Rendering|Material|SetScalarParameterValue (Variables|Default|GetTileMaterialInstance) "YOffset" (.y _returnvalue_2) :!class /Script/Engine.MaterialInstanceDynamic))))