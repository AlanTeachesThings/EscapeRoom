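; Single-press keypad button for the escape room that carries a KeypadNumber.
; One tick after the parent BeginPlay, it copies that number into ValueToSendOnPress, the value for a press.
; CreateDynamicMatInstance builds a Keypad_M instance for the mesh, using the number's modulo and integer division by 3 as X and Y offsets, so one material serves every key.
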(event EventBeginPlay
  (|CallParentFunction)
  (Utilities|FlowControl|DelayUntilNextTick)
  (Variables|Default|SetValueToSendOnPress (Variables|Default|GetKeypadNumber)))

(event Collision|EventActorBeginOverlap
  (params (OtherActor :type Actor%20Object%20Reference)))

(event EventTick
  (params (DeltaSeconds :type Float%20%28single-precision%29)))

(event EventAddHighlight
  (|CallParentFunction))

(fn ConstructionScript
  (|CallParentFunction))

(fn CreateDynamicMatInstance
  (bind _keypadnumber (Variables|Default|GetKeypadNumber))
  (bind _returnvalue (- _keypadnumber 0))
  (bind _returnvalue_2 (Rendering|Material|CreateDynamicMaterialInstance "/Game/EscapeRoom/Interactions/Panels/Keypad/textures/Keypad_M.Keypad_M" "None" "None" :!class /Script/Engine.KismetMaterialLibrary))
  (Rendering|Material|SetScalarParameterValue _returnvalue_2 "XOffset" (Math|Conversions|ToFloat(Integer) (Math|Integer|%(Integer) _returnvalue 3)) :!class /Script/Engine.MaterialInstanceDynamic)
  (Rendering|Material|SetScalarParameterValue _returnvalue_2 "YOffset" (Math|Conversions|ToFloat(Integer) (/ _returnvalue 3)) :!class /Script/Engine.MaterialInstanceDynamic)
  (Rendering|Material|SetMaterial (Variables|Default|GetStaticMesh) 0 _returnvalue_2))