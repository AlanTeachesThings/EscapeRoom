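; Toggle switch interactable for the escape room, with two states, on and off.
; Each interaction flips IsOn and calls OnActions or OffActions, which are empty events here.
; It then removes the highlight and sends ValueWhenOn or ValueWhenOff to targeted objects according to the new state.
; The interaction ends immediately on the instigating character, so each use is a single toggle.
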(event Custom|OnActions)

(event Custom|OffActions)

(event EventInteractStart
  (params (InstigatingCharacter :type BP%20First%20Person%20Character%20Object%20Reference))
  (if (Variables|Default|GetisOn)
    (Variables|Default|SetisOn false)
    (CallFunction|OffActions)
    (else
      (Variables|Default|SetisOn true)
      (CallFunction|OnActions)))
  (CallFunction|RemoveHighlight)
  (CallFunction|SendValuetoTargetedObjects (Math|Integer|SelectInt (Variables|InteractSystem|GetValueWhenOn) (Variables|InteractSystem|GetValueWhenOff) (Variables|Default|GetisOn)))
  (Default|EndInteraction InstigatingCharacter))

(fn ConstructionScript
  (|CallParentFunction))