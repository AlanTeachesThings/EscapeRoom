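; Sliding tile puzzle panel for the escape room, built on a parent panel class with a lock component.
; Construction fills a grid with tile slots around one empty space, and shared setup (also run at BeginPlay) gives each tile movement limits, a texture slice and a target position.
; A received value makes every tile re-resolve its lock, with a DoOnce reset next tick preventing feedback loops.
; Unlocking force-stops panel interaction.
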(event Custom|SetupTiles
  (bind _gridsize (Variables|SlidingTilePanelSetup|GetGridSize))
  (bind _gridspacing (Variables|SlidingTilePanelSetup|GetGridSpacing))
  (bind _gridspacing_2 (Variables|SlidingTilePanelSetup|GetGridSpacing))
  (bind _texturedivisions (Variables|SlidingTilePanelSetup|GetTextureDivisions))
  (bind _returnvalue (/ 1.0 _texturedivisions))
  ;[0.15 0.15 0.15 0.5] Extra Panel Setup
  (bind (_keypin _valuepin) (Utilities|Map|ForEachLoop(Map) (Variables|Default|GetIndicesByGridPosition))
    (:then
      (Utilities|FlowControl|Sequence
        (:then_0
          ;;[0.15 0.15 0.15 0.5] Print Debug Text
          (Rendering|Components|TextRender|SetText (Variables|/Game/EscapeRoom/Interactions/SlidingTile/SlidingTile_BP.SlidingTile_BP_C|GetDebugTextRender (.AsSliding%20Tile%20BP (Utilities|Casting|CastToSlidingTile_BP (CallFunction|GetPanelInteractablebyKey _valuepin)))) (Utilities|Text|ToText(String) _keypin)))
        (:then_1
          ;;[0.15 0.15 0.15 0.5] Set Movement Limits based on Grid Position
          (Utilities|FlowControl|Sequence
            (:then_0
              (Variables|/Game/EscapeRoom/Interactions/SlidingTile/SlidingTile_BP.SlidingTile_BP_C|SetRightLimit (.AsSliding%20Tile%20BP (Utilities|Casting|CastToSlidingTile_BP (CallFunction|GetPanelInteractablebyKey _valuepin))) (Math|Vector|MakeVector (* (- (.x _gridsize) (.X (Math|Vector2D|BreakVector2D _keypin))) _gridspacing_2) 0.0 0.0))
              (Variables|/Game/EscapeRoom/Interactions/SlidingTile/SlidingTile_BP.SlidingTile_BP_C|SetLeftLimit (.AsSliding%20Tile%20BP (Utilities|Casting|CastToSlidingTile_BP (CallFunction|GetPanelInteractablebyKey _valuepin))) (Math|Vector|MakeVector (* (- 0.0 (.X (Math|Vector2D|BreakVector2D _keypin))) _gridspacing) 0.0 0.0)))
            (:then_1
              (Variables|/Game/EscapeRoom/Interactions/SlidingTile/SlidingTile_BP.SlidingTile_BP_C|SetUpperLimit (.AsSliding%20Tile%20BP (Utilities|Casting|CastToSlidingTile_BP (CallFunction|GetPanelInteractablebyKey _valuepin))) (Math|Vector|MakeVector 0.0 0.0 (* (- (.y _gridsize) (.Y (Math|Vector2D|BreakVector2D _keypin))) _gridspacing_2)))
              (Variables|/Game/EscapeRoom/Interactions/SlidingTile/SlidingTile_BP.SlidingTile_BP_C|SetLowerLimit (.AsSliding%20Tile%20BP (Utilities|Casting|CastToSlidingTile_BP (CallFunction|GetPanelInteractablebyKey _valuepin))) (Math|Vector|MakeVector 0.0 0.0 (* (- 0.0 (.Y (Math|Vector2D|BreakVector2D _keypin))) _gridspacing))))))
        (:then_2
          ;;[0.15 0.15 0.15 0.5] Set up Textures
          (Rendering|Material|SetTextureParameterValue (Variables|/Game/EscapeRoom/Interactions/SlidingTile/SlidingTile_BP.SlidingTile_BP_C|GetTileMaterialInstance (.AsSliding%20Tile%20BP (Utilities|Casting|CastToSlidingTile_BP (CallFunction|GetPanelInteractablebyKey _valuepin)))) "TileTexture" (Variables|SlidingTilePanelSetup|GetTileTexture))
          (Rendering|Material|SetScalarParameterValue (Variables|/Game/EscapeRoom/Interactions/SlidingTile/SlidingTile_BP.SlidingTile_BP_C|GetTileMaterialInstance (.AsSliding%20Tile%20BP (Utilities|Casting|CastToSlidingTile_BP (CallFunction|GetPanelInteractablebyKey _valuepin)))) "XOffset" (* _returnvalue (.X (Math|Vector2D|BreakVector2D (.Value (Utilities|Map|Find (Variables|SlidingTilePanelSetup|GetTilePositionToTargetPosition) _keypin))))) :!class /Script/Engine.MaterialInstanceDynamic)
          (Rendering|Material|SetScalarParameterValue (Variables|/Game/EscapeRoom/Interactions/SlidingTile/SlidingTile_BP.SlidingTile_BP_C|GetTileMaterialInstance (.AsSliding%20Tile%20BP (Utilities|Casting|CastToSlidingTile_BP (CallFunction|GetPanelInteractablebyKey _valuepin)))) "YOffset" (* _returnvalue (- (.y (Variables|SlidingTilePanelSetup|GetGridSize)) (.Y (Math|Vector2D|BreakVector2D (.Value (Utilities|Map|Find (Variables|SlidingTilePanelSetup|GetTilePositionToTargetPosition) _keypin)))))) :!class /Script/Engine.MaterialInstanceDynamic))
        (:then_3
          ;;[0.15 0.15 0.15 0.5] Set Target Position
          (bind _output_get (Variables|/Game/EscapeRoom/Interactions/SlidingTile/SlidingTile_BP.SlidingTile_BP_C|SetTargetPosition (.AsSliding%20Tile%20BP (Utilities|Casting|CastToSlidingTile_BP (CallFunction|GetPanelInteractablebyKey _valuepin))) (* (- (.Value (Utilities|Map|Find (Variables|SlidingTilePanelSetup|GetTilePositionToTargetPosition) _keypin)) _keypin) (Variables|SlidingTilePanelSetup|GetGridSpacing))))
          (Transformation|SetRelativeLocation (Variables|/Game/EscapeRoom/Interactions/SlidingTile/SlidingTile_BP.SlidingTile_BP_C|GetDebugTargetMarker (.AsSliding%20Tile%20BP (Utilities|Casting|CastToSlidingTile_BP (CallFunction|GetPanelInteractablebyKey _valuepin)))) (Math|Vector|MakeVector (.x _output_get) 0.0 (.y _output_get)) false false))))))

(event EventValue
  (params (SendingInteractable :type Interactable%20Base%20BP%20Object%20Reference) (Value :type Integer))
  ;[0.15 0.15 0.15 0.5] Receive Value: Trigger ALL tiles to resolve lock, but block infinite loop
  (Utilities|FlowControl|Sequence
    (:then_0
      (Utilities|FlowControl|DoOnce false :!label _label
        (:Completed
          (bind _values (Utilities|Map|Values (Variables|Default|GetPanelComponents)))
          (for _array_element _values
            (bind _assliding_tile_bp (Utilities|Casting|CastToSlidingTile_BP (Variables|/Script/Engine.ChildActorComponent|GetChildActor _array_element)))
            (Default|ForceResolveLock _assliding_tile_bp)))))
    (:then_1
      (Default|ReceiveValue (Variables|Default|GetLockComponent) SendingInteractable Value))
    (:then_2
      (Utilities|FlowControl|DelayUntilNextTick)
      (goto _label Reset))))

(event EventBeginPlay
  (bind _gridsize (Variables|SlidingTilePanelSetup|GetGridSize))
  (bind _gridspacing (Variables|SlidingTilePanelSetup|GetGridSpacing))
  (bind _gridspacing_2 (Variables|SlidingTilePanelSetup|GetGridSpacing))
  (bind _texturedivisions (Variables|SlidingTilePanelSetup|GetTextureDivisions))
  (bind _returnvalue (/ 1.0 _texturedivisions))
  (|CallParentFunction)
  (Utilities|FlowControl|DelayUntilNextTick)
  (Utilities|FlowControl|Sequence
    (:then_0
      ;[0.15 0.15 0.15 0.5] Extra Panel Setup
      (bind (_keypin _valuepin) (Utilities|Map|ForEachLoop(Map) (Variables|Default|GetIndicesByGridPosition))
        (:then
          (Utilities|FlowControl|Sequence
            (:then_0
              ;;[0.15 0.15 0.15 0.5] Print Debug Text
              (Rendering|Components|TextRender|SetText (Variables|/Game/EscapeRoom/Interactions/SlidingTile/SlidingTile_BP.SlidingTile_BP_C|GetDebugTextRender (.AsSliding%20Tile%20BP (Utilities|Casting|CastToSlidingTile_BP (CallFunction|GetPanelInteractablebyKey _valuepin)))) (Utilities|Text|ToText(String) _keypin)))
            (:then_1
              ;;[0.15 0.15 0.15 0.5] Set Movement Limits based on Grid Position
              (Utilities|FlowControl|Sequence
                (:then_0
                  (Variables|/Game/EscapeRoom/Interactions/SlidingTile/SlidingTile_BP.SlidingTile_BP_C|SetRightLimit (.AsSliding%20Tile%20BP (Utilities|Casting|CastToSlidingTile_BP (CallFunction|GetPanelInteractablebyKey _valuepin))) (Math|Vector|MakeVector (* (- (.x _gridsize) (.X (Math|Vector2D|BreakVector2D _keypin))) _gridspacing_2) 0.0 0.0))
                  (Variables|/Game/EscapeRoom/Interactions/SlidingTile/SlidingTile_BP.SlidingTile_BP_C|SetLeftLimit (.AsSliding%20Tile%20BP (Utilities|Casting|CastToSlidingTile_BP (CallFunction|GetPanelInteractablebyKey _valuepin))) (Math|Vector|MakeVector (* (- 0.0 (.X (Math|Vector2D|BreakVector2D _keypin))) _gridspacing) 0.0 0.0)))
                (:then_1
                  (Variables|/Game/EscapeRoom/Interactions/SlidingTile/SlidingTile_BP.SlidingTile_BP_C|SetUpperLimit (.AsSliding%20Tile%20BP (Utilities|Casting|CastToSlidingTile_BP (CallFunction|GetPanelInteractablebyKey _valuepin))) (Math|Vector|MakeVector 0.0 0.0 (* (- (.y _gridsize) (.Y (Math|Vector2D|BreakVector2D _keypin))) _gridspacing_2)))
                  (Variables|/Game/EscapeRoom/Interactions/SlidingTile/SlidingTile_BP.SlidingTile_BP_C|SetLowerLimit (.AsSliding%20Tile%20BP (Utilities|Casting|CastToSlidingTile_BP (CallFunction|GetPanelInteractablebyKey _valuepin))) (Math|Vector|MakeVector 0.0 0.0 (* (- 0.0 (.Y (Math|Vector2D|BreakVector2D _keypin))) _gridspacing))))))
            (:then_2
              ;;[0.15 0.15 0.15 0.5] Set up Textures
              (Rendering|Material|SetTextureParameterValue (Variables|/Game/EscapeRoom/Interactions/SlidingTile/SlidingTile_BP.SlidingTile_BP_C|GetTileMaterialInstance (.AsSliding%20Tile%20BP (Utilities|Casting|CastToSlidingTile_BP (CallFunction|GetPanelInteractablebyKey _valuepin)))) "TileTexture" (Variables|SlidingTilePanelSetup|GetTileTexture))
              (Rendering|Material|SetScalarParameterValue (Variables|/Game/EscapeRoom/Interactions/SlidingTile/SlidingTile_BP.SlidingTile_BP_C|GetTileMaterialInstance (.AsSliding%20Tile%20BP (Utilities|Casting|CastToSlidingTile_BP (CallFunction|GetPanelInteractablebyKey _valuepin)))) "XOffset" (* _returnvalue (.X (Math|Vector2D|BreakVector2D (.Value (Utilities|Map|Find (Variables|SlidingTilePanelSetup|GetTilePositionToTargetPosition) _keypin))))) :!class /Script/Engine.MaterialInstanceDynamic)
              (Rendering|Material|SetScalarParameterValue (Variables|/Game/EscapeRoom/Interactions/SlidingTile/SlidingTile_BP.SlidingTile_BP_C|GetTileMaterialInstance (.AsSliding%20Tile%20BP (Utilities|Casting|CastToSlidingTile_BP (CallFunction|GetPanelInteractablebyKey _valuepin)))) "YOffset" (* _returnvalue (- (.y (Variables|SlidingTilePanelSetup|GetGridSize)) (.Y (Math|Vector2D|BreakVector2D (.Value (Utilities|Map|Find (Variables|SlidingTilePanelSetup|GetTilePositionToTargetPosition) _keypin)))))) :!class /Script/Engine.MaterialInstanceDynamic))
            (:then_3
              ;;[0.15 0.15 0.15 0.5] Set Target Position
              (bind _output_get (Variables|/Game/EscapeRoom/Interactions/SlidingTile/SlidingTile_BP.SlidingTile_BP_C|SetTargetPosition (.AsSliding%20Tile%20BP (Utilities|Casting|CastToSlidingTile_BP (CallFunction|GetPanelInteractablebyKey _valuepin))) (* (- (.Value (Utilities|Map|Find (Variables|SlidingTilePanelSetup|GetTilePositionToTargetPosition) _keypin)) _keypin) (Variables|SlidingTilePanelSetup|GetGridSpacing))))
              (Transformation|SetRelativeLocation (Variables|/Game/EscapeRoom/Interactions/SlidingTile/SlidingTile_BP.SlidingTile_BP_C|GetDebugTargetMarker (.AsSliding%20Tile%20BP (Utilities|Casting|CastToSlidingTile_BP (CallFunction|GetPanelInteractablebyKey _valuepin)))) (Math|Vector|MakeVector (.x _output_get) 0.0 (.y _output_get)) false false))))))
    (:then_1
      (Variables|/Game/EscapeRoom/Objects/LockComponent.LockComponent_C|SetLockStyle (Variables|Default|GetLockComponent) "NewEnumerator2"))))

(event EventUnlockActions
  (|CallParentFunction)
  (CallFunction|ForceStopPanelInteraction))

(fn ConstructionScript
  (bind _gridspacing (Variables|SlidingTilePanelSetup|GetGridSpacing))
  (bind _gridsize (Variables|SlidingTilePanelSetup|GetGridSize))
  (bind _gridspacing_2 (Variables|SlidingTilePanelSetup|GetGridSpacing))
  (bind _returnvalue (* _gridsize _gridspacing_2))
  (bind _returnvalue_2 (/ _returnvalue "(X=2.000000,Y=2.000000)"))
  (Utilities|FlowControl|Sequence
    (:then_0
      ;[0.15 0.15 0.15 0.5] Construct Grid of Tiles
      (Utilities|Map|Clear (Variables|Default|GetPanelSlotSetup))
      (for _index (range 0 (Math|Float|Truncate (.x (Variables|SlidingTilePanelSetup|GetGridSize))))
        (for _index_2 (range 0 (Math|Float|Truncate (.y (Variables|SlidingTilePanelSetup|GetGridSize))))
          (if (Utilities|Operators|NotEqual(!=) (Variables|SlidingTilePanelSetup|GetEmptySpace) (Math|Vector2D|MakeVector2D (Math|Conversions|ToFloat(Integer) _index) (Math|Conversions|ToFloat(Integer) _index_2)) 0.0)
            (Utilities|Map|Add (Variables|Default|GetPanelSlotSetup) (+ _index_2 (* _index 10)) (Utilities|Struct|MakePanelSlot (Variables|SlidingTilePanelSetup|GetPanelClass) (Math|Transform|MakeTransform (Math|Vector|MakeVector (- (* _index _gridspacing) (.x _returnvalue_2)) 0.0 (- (* _gridspacing _index_2) (.y _returnvalue_2))) "0, 0, 0" "1.000000,1.000000,1.000000") 0 0 0 0 0 0))
            (Utilities|Map|Add (Variables|Default|GetIndicesByGridPosition) (Math|Vector2D|MakeVector2D (Math|Conversions|ToFloat(Integer) _index) (Math|Conversions|ToFloat(Integer) _index_2)) (+ _index_2 (* _index 10)))))))
    (:then_1
      (|CallParentFunction))
    (:then_2
      (CallFunction|SetupTiles))))

(fn GetPanelInteractablebyKey
  (params (Key :type Integer%20%28by%20ref%29))
  (return (|CallParentFunction Key)))