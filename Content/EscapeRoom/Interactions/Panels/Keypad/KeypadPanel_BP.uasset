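; Keypad panel Blueprint for escape room interactions, built on a parent panel class and acting as a combination lock.
; On BeginPlay it sets the lock operation mode and maps each combination entry by index into KeyValuesByComponentID before running parent logic.
; At construction and BeginPlay, it pushes KeypadNumbers values into matching child-actor KeypadButton_BP components and has each create a dynamic material instance.
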(event EventBeginPlay
  (Variables|Default|SetLockOperation "NewEnumerator3")
  (for (_array_element _array_index) (Variables|Default|GetLockCombination)
    (Utilities|Map|Add (Variables|Default|GetKeyValuesByComponentID) _array_index _array_element))
  (|CallParentFunction)
  (CallFunction|SetKeypadButtonMaterials))

(fn ConstructionScript
  (|CallParentFunction)
  (CallFunction|SetKeypadButtonMaterials))

(fn SetKeypadButtonMaterials
  (bind (_keypin _valuepin) (Utilities|Map|ForEachLoop(Map) (Variables|Default|GetKeypadNumbers))
    (:then
      (if (.ReturnValue (Utilities|Map|Find (Variables|Default|GetPanelComponents) _keypin))
        (bind _askeypad_button_bp (Utilities|Casting|CastToKeypadButton_BP (Variables|/Script/Engine.ChildActorComponent|GetChildActor (.Value (Utilities|Map|Find (Variables|Default|GetPanelComponents) _keypin)))))
        (Variables|/Game/EscapeRoom/Interactions/Buttons/SinglePress/KeypadButton_BP.KeypadButton_BP_C|SetKeypadNumber _askeypad_button_bp _valuepin)
        (Default|CreateDynamicMatInstance _askeypad_button_bp)))))