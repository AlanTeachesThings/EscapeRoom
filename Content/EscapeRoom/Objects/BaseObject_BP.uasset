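; Base escape-room object that locks and unlocks according to key values received from sending interactables.
; Each received value is checked against KeyValues by the LockOperation mode: Any, All, their per-sender Exclusive variants, or Specific sender-value pairs.
; Exclusive and Specific modes keep only each sender's latest signal.
; ResolveUnlock gates the Lock and Unlock events through paired DoOnce nodes, and Unlock reports success to targeting interactables.
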(event Custom|ResolveUnlock
  (if (Variables|Default|GetShouldUnlock)
    (Utilities|FlowControl|DoOnce false :!label _label
      (:Completed
        (CallFunction|Unlock)
        (goto _label_2 Reset)))
    (else
      (Utilities|FlowControl|DoOnce (Variables|Default|GetLockedAtStart) :!label _label_2
        (:Completed
          (CallFunction|Lock)
          (goto _label Reset))))))

(event Custom|Lock)

(event Custom|Unlock
  (bind _keys (Utilities|Map|Keys (Variables|Default|GetKeyValuesByTargetingInteractable)))
  (for _array_element _keys
    (Default|ReportUnlockSuccesful _array_element self)))

(event EventValue
  (params (SendingInteractable :type Interactable%20Base%20BP%20Object%20Reference) (Value :type Integer))
  (bind _keystatuses (Variables|Default|GetKeyStatuses))
  (bind _receivedsignals (Variables|Default|GetReceivedSignals))
  (bind _keystatuses_2 (Variables|Default|GetKeyStatuses))
  (bind _keystatuses_3 (Variables|Default|GetKeyStatuses))
  (switch Utilities|FlowControl|Switch|SwitchonObjectLockOperations (Variables|Default|GetLockOperation)
    (:NewEnumerator0
      ;[0.15 0.15 0.15 0.5] Any: If received value matches ANY key value, should unlock
      (Variables|Default|SetShouldUnlock false)
      (for _array_element (Variables|InteractSystem|GetKeyValues)
        (if (== (.key _array_element) Value)
          (Variables|Default|SetShouldUnlock true)))
      (CallFunction|ResolveUnlock))
    (:NewEnumerator4
      ;[0.15 0.15 0.15 0.5] Exclusive: if any received value matches, but only allow one per sender
      (Variables|Default|SetShouldUnlock false)
      (CallFunction|ReceiveExclusiveSignal Value SendingInteractable)
      (for _array_element_2 (Variables|Default|GetReceivedSignals)
        (for _array_element_3 (Variables|InteractSystem|GetKeyValues)
          (if (== (.key _array_element_3) (.key _array_element_2))
            (Variables|Default|SetShouldUnlock true))))
      (CallFunction|ResolveUnlock))
    (:NewEnumerator1
      ;[0.15 0.15 0.15 0.5] All: All signals must be received at some point to unlock
      (Variables|Default|SetShouldUnlock true)
      (Utilities|Array|Add _receivedsignals (Utilities|Struct|MakeKeySenders Value SendingInteractable))
      (bind _array_element_4 (Utilities|Array|ForEachLoopwithBreak _receivedsignals)
        (:LoopBody
          (bind (_array_element_5 _array_index) (Utilities|Array|ForEachLoopwithBreak (Variables|InteractSystem|GetKeyValues) :!label _label)
            (:LoopBody
              (if (== (.key _array_element_4) (.key _array_element_5))
                (if (not (Utilities|Array|Get(acopy) _keystatuses_2 _array_index))
                  (Utilities|Array|SetArrayElem _keystatuses_2 _array_index true)
                  (goto _label Break))))))
        (:Completed
          (for _array_element_6 (Variables|Default|GetKeyStatuses)
            (if (not _array_element_6)
              (Variables|Default|SetShouldUnlock false)))
          (CallFunction|ResolveUnlock))))
    (:NewEnumerator5
      ;[0.15 0.15 0.15 0.5] All Exclusive: All signals must be received FROM DIFFERENT SENDERS at some point to unlock
      (Variables|Default|SetShouldUnlock true)
      (CallFunction|ReceiveExclusiveSignal Value SendingInteractable)
      (for (_ _array_index_2) _keystatuses_3
        (Utilities|Array|SetArrayElem _keystatuses_3 _array_index_2 false))
      (bind _array_element_7 (Utilities|Array|ForEachLoopwithBreak (Variables|Default|GetReceivedSignals))
        (:LoopBody
          (bind (_array_element_8 _array_index_3) (Utilities|Array|ForEachLoopwithBreak (Variables|InteractSystem|GetKeyValues) :!label _label_2)
            (:LoopBody
              (if (== (.key _array_element_7) (.key _array_element_8))
                (if (not (Utilities|Array|Get(acopy) _keystatuses _array_index_3))
                  (Utilities|Array|SetArrayElem _keystatuses _array_index_3 true)
                  (goto _label_2 Break))))))
        (:Completed
          (for _array_element_9 (Variables|Default|GetKeyStatuses)
            (if (not _array_element_9)
              (Variables|Default|SetShouldUnlock false)))
          (CallFunction|ResolveUnlock))))
    (:NewEnumerator2
      ;[0.15 0.15 0.15 0.5] Specific: Only Unlock if receiving specific signals from specific senders
      (Variables|Default|SetShouldUnlock true)
      (CallFunction|ReceiveExclusiveSignal Value SendingInteractable)
      (for _array_element_10 (Variables|Default|GetReceivedSignals)
        (for (_array_element_11 _array_index_4) (Variables|InteractSystem|GetKeyValues)
          (if (== (.interactable _array_element_11) (.interactable _array_element_10))
            (Utilities|Array|SetArrayElem (Variables|Default|GetKeyStatuses) _array_index_4 (== (.key _array_element_11) (.key _array_element_10))))))
      (for _array_element_12 (Variables|Default|GetKeyStatuses)
        (if (not _array_element_12)
          (Variables|Default|SetShouldUnlock false)))
      (CallFunction|ResolveUnlock))))

(event EventBeginPlay
  ;[0.15 0.15 0.15 0.5] BeginPlay
  (for _array_element (Variables|InteractSystem|GetKeyValues)
    (Utilities|Array|Add (Variables|Default|GetKeyStatuses) false)))

(fn ConstructionScript)

(fn ReceiveExclusiveSignal
  (params (Value :type Integer) (SendingInteractable :type Interactable%20Base%20BP%20Object%20Reference))
  (bind _receivedsignals (Variables|Default|GetReceivedSignals))
  (for (_array_element _array_index) (Variables|Default|GetReceivedSignals)
    (if (== (.interactable _array_element) SendingInteractable)
      (LocalVariables|SetMatchFound true)
      (LocalVariables|SetMatchIndex _array_index)))
  (if (LocalVariables|GetMatchFound)
    (Utilities|Array|SetArrayElem _receivedsignals (LocalVariables|GetMatchIndex) (Utilities|Struct|MakeKeySenders Value SendingInteractable))
    (else
      (Utilities|Array|Add _receivedsignals (Utilities|Struct|MakeKeySenders Value SendingInteractable)))))