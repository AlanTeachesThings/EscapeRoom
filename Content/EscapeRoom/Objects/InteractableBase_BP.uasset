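; InteractableBase_BP is the base Blueprint for interactable objects in the escape room, providing highlighting and an interaction event interface.
; AddHighlight attaches a Niagara system to every static and skeletal mesh component, using a separate system for each type, and stores them for RemoveHighlight to destroy.
; Its interaction events for start, directional control, press phases and back are empty hooks that receive the instigating character.
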(event Custom|AddHighlight
  (Utilities|FlowControl|Sequence
    (:then_0
      (for _array_element (Actor|GetComponentsByClass "/Script/Engine.StaticMeshComponent")
        (bind _returnvalue (Niagara|SpawnSystemAttached "/Game/EscapeRoom/Objects/VFX/HighlightSystemStatic_NS.HighlightSystemStatic_NS" _array_element "None" "0, 0, 0" "0, 0, 0" "KeepRelativeOffset" false))
        (Utilities|Array|Add (Variables|Default|GetHighlightSystemComponents) _returnvalue)))
    (:then_1
      (for _array_element_2 (Actor|GetComponentsByClass "/Script/Engine.SkeletalMeshComponent")
        (bind _returnvalue_2 (Niagara|SpawnSystemAttached "/Game/EscapeRoom/Objects/VFX/HighlightSystemSkeletal_NS.HighlightSystemSkeletal_NS" _array_element_2 "None" "0, 0, 0" "0, 0, 0" "KeepRelativeOffset" false))
        (Utilities|Array|Add (Variables|Default|GetHighlightSystemComponents) _returnvalue_2)))))

(event Custom|RemoveHighlight
  (for _array_element (Variables|Default|GetHighlightSystemComponents)
    (Utilities|IsValid _array_element
      (:Is%20Valid
        (Components|DestroyComponent _array_element))))
  (Utilities|Array|Clear (Variables|Default|GetHighlightSystemComponents)))

(event Custom|InteractStart
  (params (InstigatingCharacter :type BP%20First%20Person%20Character%20Object%20Reference)))

(event Custom|InteractDirectionalControl
  (params (ControlValues :type Vector%202D%20Structure) (InstigatingCharacter :type BP%20First%20Person%20Character%20Object%20Reference)))

(event Custom|InteractBack
  (params (InstigatingCharacter :type BP%20First%20Person%20Character%20Object%20Reference)))

(event Custom|InteractPressTick
  (params (InstigatingCharacter :type BP%20First%20Person%20Character%20Object%20Reference)))

(event Custom|InteractPressStart
  (params (InstigatingCharacter :type BP%20First%20Person%20Character%20Object%20Reference)))

(event Custom|InteractPressEnd
  (params (InstigatingCharacter :type BP%20First%20Person%20Character%20Object%20Reference)))

(fn ConstructionScript)