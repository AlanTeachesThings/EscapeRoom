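; Furniture helper actor for the escape room that builds movable mesh parts from a configurable Helpers array.
; AddHelpers destroys all child actor components, then spawns one EasyMeshMover_BP per entry, passing mesh, target transform, curve and lock state.
; The construction script can preview parts at their targets via ShowHelpersAtTarget, while BeginPlay rebuilds them with that preview off.
; Value events from interactables are forwarded to every mover.
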(event EventBeginPlay
  (CallFunction|AddHelpers false))

(event Collision|EventActorBeginOverlap
  (params (OtherActor :type Actor%20Object%20Reference)))

(event EventTick
  (params (DeltaSeconds :type Float%20%28single-precision%29)))

(event EventValue
  (params (SendingInteractable :type Interactable%20Base%20BP%20Object%20Reference) (Value :type Integer))
  (for _array_element (Variables|Default|GetMoverComponents)
    (bind _aseasy_mesh_mover_bp (Utilities|Casting|CastToEasyMeshMover_BP (Variables|/Script/Engine.ChildActorComponent|GetChildActor _array_element)))
    (Default|ReceiveValue _aseasy_mesh_mover_bp SendingInteractable Value)))

(fn ConstructionScript
  (CallFunction|AddHelpers (Variables|Default|GetShowHelpersAtTarget)))

(fn AddHelpers
  (params (ShowAtTarget :type Boolean))
  (for _array_element (Variables|Default|GetMoverComponents)
    (Components|DestroyComponent _array_element))
  (Utilities|Array|Clear (Variables|Default|GetMoverComponents))
  (for _array_element_2 (Actor|GetComponentsByClass "/Script/Engine.ChildActorComponent")
    (Components|DestroyComponent _array_element_2))
  (for _array_element_3 (Variables|Default|GetHelpers)
    (bind _returnvalue (AddComponent|AddChildActorComponent false (Math|Transform|MakeTransform (.relativelocation _array_element_3) (.relativerotation _array_element_3) "1.000000,1.000000,1.000000")))
    (ChildActorComponent|SetChildActorClass _returnvalue "/Game/EscapeRoom/Interactions/Furniture/FurnitureHelpers/EasyMeshMover_BP.EasyMeshMover_BP_C")
    (Utilities|Array|Add (Variables|Default|GetMoverComponents) _returnvalue)
    (bind _aseasy_mesh_mover_bp (Utilities|Casting|CastToEasyMeshMover_BP (Variables|/Script/Engine.ChildActorComponent|GetChildActor _returnvalue)))
    (Variables|/Game/EscapeRoom/Interactions/Furniture/FurnitureHelpers/EasyMeshMover_BP.EasyMeshMover_BP_C|SetMeshToMove _aseasy_mesh_mover_bp (.meshtomove _array_element_3))
    (Variables|/Game/EscapeRoom/Interactions/Furniture/FurnitureHelpers/EasyMeshMover_BP.EasyMeshMover_BP_C|SetTargetLocation _aseasy_mesh_mover_bp (.targetlocation _array_element_3))
    (Variables|/Game/EscapeRoom/Interactions/Furniture/FurnitureHelpers/EasyMeshMover_BP.EasyMeshMover_BP_C|SetTargetRotation _aseasy_mesh_mover_bp (.targetrotation _array_element_3))
    (Variables|/Game/EscapeRoom/Interactions/Furniture/FurnitureHelpers/EasyMeshMover_BP.EasyMeshMover_BP_C|SetCurve _aseasy_mesh_mover_bp (.curve _array_element_3))
    (Variables|/Game/EscapeRoom/Interactions/InteractableBase_BP.InteractableBase_BP_C|SetisLocked _aseasy_mesh_mover_bp (.islocked _array_element_3))
    (Default|SetMesh _aseasy_mesh_mover_bp ShowAtTarget)))