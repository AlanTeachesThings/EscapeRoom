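; Escape room door Blueprint secured by a tumbler lock, opening and closing as it unlocks and locks.
; On BeginPlay it passes its Combination to the LockComponent and sets a fixed lock style.
; The UnlockActions and LockActions events play one-shot open and close animations on the Door.
; The construction script only calls its parent's.
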(event EventBeginPlay
  (bind _lockcomponent (Variables|Default|GetLockComponent))
  (Variables|/Game/EscapeRoom/Objects/LockComponent.LockComponent_C|SetCombination _lockcomponent (Variables|Default|GetCombination))
  (Variables|/Game/EscapeRoom/Objects/LockComponent.LockComponent_C|SetLockStyle _lockcomponent "NewEnumerator6"))

(event EventUnlockActions
  (Components|Animation|PlayAnimation (Variables|Default|GetDoor) "/Game/EscapeRoom/Objects/Door/Anim/DoorOpen.DoorOpen" false))

(event EventLockActions
  (Components|Animation|PlayAnimation (Variables|Default|GetDoor) "/Game/EscapeRoom/Objects/Door/Anim/DoorClose.DoorClose" false))

(fn ConstructionScript
  (|CallParentFunction))