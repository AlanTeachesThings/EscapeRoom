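; Escape room door that opens only for a specific combination of sources and their values, set through the SpecificCombination map.
; On BeginPlay it copies the map's keys into the LockComponent as expected sources and its values as the combination, then sets the lock style.
; The unlock and lock events play the door's open and close animations without looping.
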(event EventBeginPlay
  (bind _lockcomponent (Variables|Default|GetLockComponent))
  (bind _specificcombination (Variables|Default|GetSpecificCombination))
  (bind _keys (Utilities|Map|Keys _specificcombination))
  (Variables|/Game/EscapeRoom/Objects/LockComponent.LockComponent_C|SetExpectedSources _lockcomponent _keys)
  (bind _values (Utilities|Map|Values _specificcombination))
  (Variables|/Game/EscapeRoom/Objects/LockComponent.LockComponent_C|SetCombination _lockcomponent _values)
  (Variables|/Game/EscapeRoom/Objects/LockComponent.LockComponent_C|SetLockStyle _lockcomponent "NewEnumerator2"))

(event EventUnlockActions
  (Components|Animation|PlayAnimation (Variables|Default|GetDoor) "/Game/EscapeRoom/Objects/Door/Anim/DoorOpen.DoorOpen" false))

(event EventLockActions
  (Components|Animation|PlayAnimation (Variables|Default|GetDoor) "/Game/EscapeRoom/Objects/Door/Anim/DoorClose.DoorClose" false))

(fn ConstructionScript
  (|CallParentFunction))